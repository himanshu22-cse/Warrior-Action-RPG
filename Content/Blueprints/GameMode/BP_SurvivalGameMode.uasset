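; Survival game mode Blueprint that presents wave progress and player death through on-screen UI.
; It binds to the survival state-change delegate and switches on the state, spawning countdown or plain text widgets for incoming, current, last and completed waves.
; Player death clears widgets, fades the camera out, then async-loads and shows the lose screen.
; Finishing all waves only prints a debug string.
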(event `self.ReceiveBeginPlay`
  (add `self.OnSurvialGameModeStateChanged` (delegate `OnSurvialGameModeStateChanged_Event`)))

(event `OnSurvialGameModeStateChanged_Event` :!signature `self.OnSurvialGameModeStateChanged`
  (params (CurrentState :type "EWarriorSurvialGameModeState Enum" :default "WaitSpawnNewWave"))
  (switch `EWarriorSurvialGameModeState` CurrentState
    (:`WaitSpawnNewWave`
      (`self.CreateWaveWidgetWithCountDown` "New Wave Coming In" (`self.SpawnNewWaveWaitTime`)))
    (:`SpawningNewWave`
      (`KismetSystemLibrary.Delay` 1.1)
      (`self.CreateWaveWidgetNoCountDown` (`|FormatText` "Wave {CurrentWaveCount} " (`self.CurrentWaveCount`)))
      (if (== (`self.TotalWavesToSpawn`) (`self.CurrentWaveCount`))
        (`KismetSystemLibrary.Delay` 1.1)
        (`self.CreateWaveWidgetNoCountDown` "LastWave")))
    (:`WaveCompleted`
      (`self.CreateWaveWidgetWithCountDown` (`|FormatText` "Wave {CurrentWaveCount} Completed" (`self.CurrentWaveCount`)) (`self.WaveCompletedWaitTime`)))
    (:`AllWavesDone`
      (`KismetSystemLibrary.PrintString` "Hello" true true (struct :`R` 1.0 :`G` 0.246767 :`B` 0.076611 :`A` 1.0) 5.0))
    (:`PlayerDied`
      (`WidgetLayoutLibrary.RemoveAllWidgets`)
      (`PlayerCameraManager.StartCameraFade` :`self` (`GameplayStatics.GetPlayerCameraManager` 0) :`ToAlpha` 1.0 :`Duration` 2.0 :`bHoldWhenFinished` true)
      (`KismetSystemLibrary.Delay` 2.0)
      (bind _class (`|LoadAssetClass` "/Game/Blueprints/Widgets/GameModeWidgets/WBP_LoseScreen.WBP_LoseScreen_C")
        (:`Completed`
          (bind _asuser_widget (castclass `UserWidget` _class))
          (bind _returnvalue (`|CreateWidget` _asuser_widget))
          (`UserWidget.AddToViewport` _returnvalue 0))))))

(fn `CreateWaveWidgetNoCountDown`
  (params (TextContentToDisplay :type Text))
  (bind _returnvalue (`|CreateWidget` "/Game/Blueprints/Widgets/GameModeWidgets/WBP_WaveTextWithNoCountdown.WBP_WaveTextWithNoCountdown_C"))
  (`UserWidget.AddToViewport` _returnvalue 0)
  (`TextBlock.SetText` (`/Game/Blueprints/Widgets/GameModeWidgets/WBP_WaveTextWithNoCountdown.TextBlock_WaveText` _returnvalue) (`local.TextContentToDisplay`)))

(fn `CreateWaveWidgetWithCountDown`
  (params (`Text Content To Display` :type Text) (InTotalCountDownTime :type "Float (double-precision)"))
  (bind _returnvalue (`|CreateWidget` "/Game/Blueprints/Widgets/GameModeWidgets/WBP_WaveTextWithCountdown.WBP_WaveTextWithCountdown_C"))
  (`UserWidget.AddToViewport` _returnvalue 0)
  (`TextBlock.SetText` (`/Game/Blueprints/Widgets/GameModeWidgets/WBP_WaveTextWithCountdown.TextBlock_WaveText` _returnvalue) (`local.Text Content To Display`))
  (`/Game/Blueprints/Widgets/GameModeWidgets/WBP_WaveTextWithCountdown.StartCountDown` _returnvalue (`local.InTotalCountDownTime`)))

(fn `UserConstructionScript`)