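; Gameplay cue that gives audio and visual feedback when a hero successfully blocks.
; On execute it plays a magic shield sound at the target actor's location.
; It also spawns a Niagara block impact at the MagicShieldSocket location on the cue's target attach component, unattached, then returns the parent implementation's result.
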(fn `OnExecute`
  (params (MyTarget :type "Actor Object Reference") (Parameters :type "GameplayCueParameters Structure (by ref)"))
  (returns (ReturnValue :type Boolean))
  (`GameplayStatics.PlaySoundAtLocation` null "/Game/Assets/Sounds/Weapons/Block/SC_MagicShieldActiavte.SC_MagicShieldActiavte" (`Actor.K2_GetActorLocation` (`local.MyTarget`)) (struct) 1.0 1.0 0.0 null null null null)
  (`NiagaraFunctionLibrary.SpawnSystemAtLocation` null "/Game/Assets/Niagara/Impact/NS_BlockImpact.NS_BlockImpact" (`SceneComponent.GetSocketLocation` (`.TargetAttachComponent` (`AbilitySystemBlueprintLibrary.BreakGameplayCueParameters` (`local.Parameters`))) "MagicShieldSocket"))
  (return (`parent.OnExecute` (`local.MyTarget`) (`local.Parameters`))))